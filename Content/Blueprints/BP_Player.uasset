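; BP_Player is the player Blueprint, moved in the world YZ plane by the Horizontal and Vertical axis inputs.
; The axis events store H and V, which Tick combines into an unnormalized direction.
; Tick adds direction times Speed and delta time to the current location (P = P0 + vt), setting it directly without sweep, so movement ignores blocking collision.
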(event `self.ReceiveBeginPlay`)

(event `InputAxis|Vertical`
  (params (AxisValue :type "Float (single-precision)"))
  (set `self.V` AxisValue))

(event `InputAxis|Horizontal`
  (params (AxisValue :type "Float (single-precision)"))
  (set `self.H` AxisValue))

(event `self.ReceiveTick`
  (params (DeltaSeconds :type "Float (single-precision)"))
  (set `self.Dir` (`KismetMathLibrary.MakeVector` 0.0 (`self.H`) (`self.V`)))
  ;[1 1 1] P
  (`self.K2_SetActorLocation` (+ (* (* (`self.Dir`) (`self.Speed`)) DeltaSeconds) (`self.K2_GetActorLocation`))))

(fn `UserConstructionScript`)